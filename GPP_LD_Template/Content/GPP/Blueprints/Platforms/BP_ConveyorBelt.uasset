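; Conveyor belt platform that carries actors resting on it along a set direction.
; Each tick it gathers the actors overlapping its Box and offsets each along the Arrow component's forward vector, scaled by Speed and frame time.
; Actors tagged "imovable" are skipped, and the movement is applied without sweep, so collisions do not block it.
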(event `self.ReceiveTick`
  (params (DeltaSeconds :type "Float (single-precision)"))
  (for _array_element (`PrimitiveComponent.GetOverlappingActors` (`self.Box`) null)
    (if (not (`self.ActorHasTag` _array_element "imovable"))
      (`self.K2_AddActorWorldOffset` _array_element (* (* DeltaSeconds (`self.Speed`)) (`KismetMathLibrary.GetForwardVector` (`SceneComponent.K2_GetComponentRotation` (`self.Arrow`)))) false false))))

(fn `UserConstructionScript`)